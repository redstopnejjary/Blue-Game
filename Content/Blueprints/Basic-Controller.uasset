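; Basic player controller that handles camera-yaw-relative movement and a dash ability for the player character.
; Dash input runs a forward line trace that blocks dashing when an obstacle is within DashMin, and requires a full recharge value.
; A valid dash snaps the character's yaw to the nearest 90-degree axis after the trace, then launches it forward.
; A timeline then updates the recharge value that gates the next dash.
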(event `self.ReceiveBeginPlay`
  ;[1 1 1] Initialisation
  (set `self.Playable Character` (`GameplayStatics.GetPlayerCharacter` 0)))

(event `InputAxis|MoveForward`
  (params (AxisValue :type "Float (single-precision)"))
  ;[0.3291 0.5957 1 1 30] Simple Movement Input
  (`Pawn.AddMovementInput` (`self.K2_GetPawn`) (`KismetMathLibrary.GetForwardVector` (`KismetMathLibrary.MakeRotator` 0.0 0.0 (.yaw (`Pawn.GetControlRotation` (`self.K2_GetPawn`))))) AxisValue false))

(event `InputAxis|MoveRight`
  (params (AxisValue :type "Float (single-precision)"))
  ;[0.3291 0.5957 1 1 30] Simple Movement Input
  (`Pawn.AddMovementInput` (`self.K2_GetPawn`) (`KismetMathLibrary.GetRightVector` (`KismetMathLibrary.MakeRotator` 0.0 0.0 (.yaw (`Pawn.GetControlRotation` (`self.K2_GetPawn`))))) AxisValue false))

(event `InputAction|Dashing`
  (params (Key :type "Key Structure"))
  ;[0.9656 1 0.166] Dashing System
  (:`Pressed`
    (bind _candash (`self.DashCheck` (`self.Playable Character`)))
    (if (and _candash (== (`self.Dash Reacharge Delay`) 1.0))
      (`self.SetCharacterNewRotation` (`self.Playable Character`))
      (bind _dash_cost (`self.Dash Execution` (`self.Playable Character`)))
      (bind (_direction _dash_recharge_track) (`Timeline|Timeline_0` :`NewTime` _dash_cost :!via `PlayFromStart`)
        (:`Update`
          (set `self.Dash Reacharge Delay` _dash_recharge_track))))))

(fn `Dash Execution`
  (params (Robot :type "Character Object Reference"))
  (returns (`Dash Cost` :type "Float (double-precision)"))
  (`Character.LaunchCharacter` Robot (* (`self.GetActorForwardVector` Robot) 5000.0) false false)
  (return 0.0))

(fn `DashCheck`
  (params (Robot :type "Character Object Reference"))
  (returns (CanDash :type Boolean))
  (locals (`Dash Min` :type "Float (double-precision)" :default 600.0))
  (bind _returnvalue (`self.K2_GetActorLocation` Robot))
  (bind _outhit (`KismetSystemLibrary.LineTraceSingle` _returnvalue (+ _returnvalue (* (`KismetMathLibrary.GetForwardVector` (`self.K2_GetActorRotation` Robot)) 1500.0)) "TraceTypeQuery1"))
  (if (and (!= (`.Distance` (`GameplayStatics.BreakHitResult` _outhit)) 0.0) (<= (`.Distance` (`GameplayStatics.BreakHitResult` _outhit)) (`local.Dash Min`)))
    (return false)
    (else
      (return true))))

(fn `SetCharacterNewRotation`
  (params (Robot :type "Character Object Reference"))
  (bind (_returnvalue_roll _returnvalue_pitch _returnvalue_yaw) (`KismetMathLibrary.BreakRotator` (`self.K2_GetActorRotation` Robot)))
  (if (and (>= _returnvalue_yaw -45.0) (< _returnvalue_yaw 45.0))
    (`self.K2_SetActorRotation` :`self` Robot)
    (return)
    (elif (and (>= _returnvalue_yaw 45.0) (< _returnvalue_yaw 135.0))
      (`self.K2_SetActorRotation` Robot (struct :`Yaw` 90.0) false)
      (return)
      (elif (or (and (>= _returnvalue_yaw 135.0) (< _returnvalue_yaw 180.0)) (and (>= _returnvalue_yaw -180.0) (< _returnvalue_yaw -135.0)))
        (`self.K2_SetActorRotation` Robot (struct :`Yaw` -180.0) false)
        (return)
        (elif (and (>= _returnvalue_yaw -135.0) (< _returnvalue_yaw -45.0))
          (`self.K2_SetActorRotation` Robot (struct :`Yaw` -90.0) false)
          (return))))))

(fn `UserConstructionScript`)